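; BP_Carrot is a carrot actor that detects when the first-person player character is in range.
; Its Box overlap events set IsOverlappingPlayer and call SetCurrentCarrot on BP_FirstPersonCharacter, passing itself and whether the overlap began or ended.
; Its Widget starts hidden, and SetWidgetVisibility exposes a toggle that the overlap events do not call themselves.
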(event `self.ReceiveBeginPlay`
  (`SceneComponent.SetVisibility` (`self.Widget`) false false)
  (set `self.IsOverlappingPlayer` false))

(event `self.Box.OnComponentBeginOverlap`
  (params (OverlappedComponent :type "PrimitiveComponent Object Reference") (OtherActor :type "Actor Object Reference") (OtherComp :type "PrimitiveComponent Object Reference") (OtherBodyIndex :type Integer) (bFromSweep :type Boolean) (SweepResult :type "HitResult Structure (by ref)"))
  (bind _asbp_first_person_character (cast `/Game/FirstPerson/Blueprints/BP_FirstPersonCharacter` OtherActor))
  (set `self.IsOverlappingPlayer` true)
  (`/Game/FirstPerson/Blueprints/BP_FirstPersonCharacter.SetCurrentCarrot` _asbp_first_person_character self true))

(event `self.Box.OnComponentEndOverlap`
  (params (OverlappedComponent :type "PrimitiveComponent Object Reference") (OtherActor :type "Actor Object Reference") (OtherComp :type "PrimitiveComponent Object Reference") (OtherBodyIndex :type Integer))
  (bind _asbp_first_person_character (cast `/Game/FirstPerson/Blueprints/BP_FirstPersonCharacter` OtherActor))
  (set `self.IsOverlappingPlayer` false)
  (`/Game/FirstPerson/Blueprints/BP_FirstPersonCharacter.SetCurrentCarrot` _asbp_first_person_character self false))

(fn `SetWidgetVisibility`
  (params (Visible :type Boolean))
  (`SceneComponent.SetVisibility` (`self.Widget`) Visible false))

(fn `UserConstructionScript`)